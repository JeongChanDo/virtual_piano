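; Piano game mode that shows a continuously updated image on an in-world screen.
; BeginPlay spawns a BP_Screen at a fixed transform and assigns a new BP_MainWidget to its widget component.
; Each Tick calls ReadFrame, defined outside this graph, then pushes ImageTexture into the widget's image brush.
; Disconnected nodes for three more screens and widgets remain but never run.
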(event `self.ReceiveBeginPlay`
  (bind _returnvalue (`|SpawnActorFromClass` "/Game/MyContent/BP_Screen.BP_Screen_C" (`KismetMathLibrary.MakeTransform` (400.0 0.0 40.0) (struct :`Pitch` 90.0 :`Yaw` 180.0)) "Undefined" "MultiplyWithRoot" null null))
  (bind _returnvalue_2 (`|CreateWidget` "/Game/MyContent/BP_MainWidget.BP_MainWidget_C"))
  (bind _output_get (set `self.MainUI` _returnvalue_2))
  (`WidgetComponent.SetWidget` (`/Game/MyContent/BP_Screen.widgetComponent` _returnvalue) _output_get))

(event `self.ReceiveTick`
  (params (DeltaSeconds :type "Float (single-precision)"))
  (`self.ReadFrame`)
  (`Image.SetBrushFromTexture` (`/Game/MyContent/BP_MainWidget.imageWidget` (`self.MainUI`)) (`self.imageTexture`) false))

(fn `UserConstructionScript`)